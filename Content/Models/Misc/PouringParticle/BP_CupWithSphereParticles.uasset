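; Cup actor that tips over at a steady rate, apparently as a test rig for pouring sphere particles.
; Tick adds RotationSpeed to local roll each frame while roll is within a range capped at 145 degrees, without delta-time scaling.
; BeginPlay overwrites TestData.csv in the project directory with a label and the speed.
; SLContactMonitorBox overlap begin and end events log the current roll without showing it on screen.
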(event OnComponentBeginOverlap(SLContactMonitorBox)
  (params (OverlappedComponent :type Primitive%20Component%20Object%20Reference) (OtherActor :type Actor%20Object%20Reference) (OtherComp :type Primitive%20Component%20Object%20Reference) (OtherBodyIndex :type Integer) (bFromSweep :type Boolean) (SweepResult :type Hit%20Result%20Structure%20%28by%20ref%29))
  (Development|PrintString (Utilities|String|ToString(Float) (.roll (Transformation|GetActorRotation))) false true "(R=0.000000,G=0.660000,B=1.000000,A=1.000000)" 1e+01))

(event OnComponentEndOverlap(SLContactMonitorBox)
  (params (OverlappedComponent :type Primitive%20Component%20Object%20Reference) (OtherActor :type Actor%20Object%20Reference) (OtherComp :type Primitive%20Component%20Object%20Reference) (OtherBodyIndex :type Integer))
  (Development|PrintString (Utilities|String|ToString(Float) (.roll (Transformation|GetActorRotation))) false true "(R=1.000000,G=0.099455,B=0.547132,A=1.000000)" 1e+01))

(event EventBeginPlay
  (Utilities|Array|Add (Variables|Default|GetData) (Utilities|String|Append "Cup,BigBowl," (Utilities|String|ToString(Float) (Variables|Default|GetRotationSpeed))))
  (Class|CSVFileManager|SaveArrayText (Class|KismetSystemLibrary|GetProjectDirectory) "TestData.csv" (Variables|Default|GetData) true))

(event Collision|EventActorBeginOverlap
  (params (OtherActor :type Actor%20Object%20Reference)))

(event EventTick
  (params (DeltaSeconds :type Float%20%28single-precision%29))
  (if (Math|Float|InRange(Float) (.roll (Transformation|GetActorRotation)) 0.0 145.0)
    (Transformation|AddActorLocalRotation (Math|Rotator|MakeRotator (Variables|Default|GetRotationSpeed) 0.0 0.0) false false)))

(fn ConstructionScript)