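; Pouring simulation actor that tilts a milk pitcher toward a blue cup and records data about the trial.
; Tick rolls the pitcher by RotationSpeed while its roll stays within the range set by MaxPouringAngle.
; The main contact box's end overlap appends a comma-separated row of names, time, pour settings, positions and particle count to DataArray, copied to DataRaws.
; Four other contact boxes flag the pour as failed on begin overlap.
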(event OnComponentBeginOverlap(SLContactMonitorBox4)
  (params (OverlappedComponent :type Primitive%20Component%20Object%20Reference) (OtherActor :type Actor%20Object%20Reference) (OtherComp :type Primitive%20Component%20Object%20Reference) (OtherBodyIndex :type Integer) (bFromSweep :type Boolean) (SweepResult :type Hit%20Result%20Structure%20%28by%20ref%29))
  (Variables|Default|SetisPouringFailed true))

(event OnComponentBeginOverlap(SLContactMonitorBox)
  (params (OverlappedComponent :type Primitive%20Component%20Object%20Reference) (OtherActor :type Actor%20Object%20Reference) (OtherComp :type Primitive%20Component%20Object%20Reference) (OtherBodyIndex :type Integer) (bFromSweep :type Boolean) (SweepResult :type Hit%20Result%20Structure%20%28by%20ref%29)))

(event OnComponentEndOverlap(SLContactMonitorBox)
  (params (OverlappedComponent :type Primitive%20Component%20Object%20Reference) (OtherActor :type Actor%20Object%20Reference) (OtherComp :type Primitive%20Component%20Object%20Reference) (OtherBodyIndex :type Integer))
  (bind _dataarray (Variables|Default|GetDataArray))
  (bind _sm_milkpitcher (Variables|Default|GetSM_MilkPitcher))
  (bind _sm_blue_cup (Variables|Default|GetSM_Blue_Cup))
  (bind _returnvalue (Transformation|GetWorldLocation _sm_milkpitcher))
  (bind _returnvalue_2 (Transformation|GetWorldLocation _sm_blue_cup))
  (Utilities|Array|AppendArray _dataarray (Utilities|Array|MakeArray (Utilities|String|Append (Utilities|GetObjectName _sm_milkpitcher) "," (Utilities|GetObjectName _sm_blue_cup) "," (Utilities|String|ToString(Float) (Utilities|Time|GetTimeSeconds)) "," (Utilities|String|ToString(Float) (Variables|Default|GetRotationSpeed)) "," (Utilities|String|ToString(Float) (Variables|Default|GetMaxPouringAngle)) "," (Utilities|String|ToString(Float) (.x _returnvalue)) "," (Utilities|String|ToString(Float) (.y _returnvalue)) "," (Utilities|String|ToString(Float) (.z _returnvalue)) "," (Utilities|String|ToString(Float) (.x _returnvalue_2)) "," (Utilities|String|ToString(Float) (.y _returnvalue_2)) "," (Utilities|String|ToString(Float) (.z _returnvalue_2)) "," (Utilities|String|ToString(Integer) (Variables|Default|GetNumberOfParticles)))))
  (Variables|Default|SetDataRaws _dataarray))

(event OnComponentBeginOverlap(SLContactMonitorBox1)
  (params (OverlappedComponent :type Primitive%20Component%20Object%20Reference) (OtherActor :type Actor%20Object%20Reference) (OtherComp :type Primitive%20Component%20Object%20Reference) (OtherBodyIndex :type Integer) (bFromSweep :type Boolean) (SweepResult :type Hit%20Result%20Structure%20%28by%20ref%29))
  (Variables|Default|SetisPouringFailed true))

(event OnComponentBeginOverlap(SLContactMonitorBox2)
  (params (OverlappedComponent :type Primitive%20Component%20Object%20Reference) (OtherActor :type Actor%20Object%20Reference) (OtherComp :type Primitive%20Component%20Object%20Reference) (OtherBodyIndex :type Integer) (bFromSweep :type Boolean) (SweepResult :type Hit%20Result%20Structure%20%28by%20ref%29))
  (Variables|Default|SetisPouringFailed true))

(event OnComponentBeginOverlap(SLContactMonitorBox3)
  (params (OverlappedComponent :type Primitive%20Component%20Object%20Reference) (OtherActor :type Actor%20Object%20Reference) (OtherComp :type Primitive%20Component%20Object%20Reference) (OtherBodyIndex :type Integer) (bFromSweep :type Boolean) (SweepResult :type Hit%20Result%20Structure%20%28by%20ref%29))
  (Variables|Default|SetisPouringFailed true))

(event EventBeginPlay)

(event Collision|EventActorBeginOverlap
  (params (OtherActor :type Actor%20Object%20Reference)))

(event EventTick
  (params (DeltaSeconds :type Float%20%28single-precision%29))
  (bind _sm_milkpitcher (Variables|Default|GetSM_MilkPitcher))
  (if (Math|Float|InRange(Float) (.roll (Variables|/Script/Engine.SceneComponent|GetRelativeRotation _sm_milkpitcher)) 0.0 (Variables|Default|GetMaxPouringAngle))
    (Transformation|AddRelativeRotation _sm_milkpitcher (Math|Rotator|MakeRotator (Variables|Default|GetRotationSpeed) 0.0 0.0) false false)))

(fn ConstructionScript)