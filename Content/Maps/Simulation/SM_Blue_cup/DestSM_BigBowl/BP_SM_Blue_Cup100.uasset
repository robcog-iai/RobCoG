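; Blueprint actor for a blue cup in a simulation map, which tracks how many particle components it contains.
; Its construction script walks all descendants of the root component and counts those whose object name starts with "particle", ignoring case.
; The total is stored in NumberOfParticles, so the count follows the component hierarchy instead of being set by hand.
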(fn ConstructionScript
  (LocalVariables|SetCountParticles 0)
  (for _array_element (Components|GetChildrenComponents (Variables|Default|GetDefaultSceneRoot) true)
    (if (Utilities|String|StartsWith (Utilities|GetObjectName _array_element) "particle")
      (Math|Integer|IncrementInt (LocalVariables|GetCountParticles))))
  (Variables|Default|SetNumberOfParticles (LocalVariables|GetCountParticles)))