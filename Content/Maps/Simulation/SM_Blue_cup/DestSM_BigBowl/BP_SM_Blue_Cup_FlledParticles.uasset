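; Automated pouring-simulation actor that fills a blue cup with physics particles, then tilts it over a big bowl and restarts the level for the next trial.
; BeginPlay sets angle and speed from a CSV row or a save-game sweep, quitting when trials run out.
; Tick drops particles, then rotates the cup to the maximum angle.
; Contact boxes count particles hit to flag failed pours and record cup/bowl data rows.
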(event OnComponentBeginOverlap(SLContactMonitorBox4)
  (params (OverlappedComponent :type Primitive%20Component%20Object%20Reference) (OtherActor :type Actor%20Object%20Reference) (OtherComp :type Primitive%20Component%20Object%20Reference) (OtherBodyIndex :type Integer) (bFromSweep :type Boolean) (SweepResult :type Hit%20Result%20Structure%20%28by%20ref%29))
  (bind _particleshittable (Variables|Default|GetParticlesHitTable))
  (if (not (Utilities|Array|ContainsItem _particleshittable OtherComp))
    (Utilities|Array|Add _particleshittable OtherComp)
    (if (>= (/ (Math|Conversions|ToFloat(Integer) (Utilities|Array|Length (Variables|Default|GetParticlesHitTable))) (Math|Conversions|ToFloat(Integer) (Variables|Default|GetNumberOfParticles))) (Variables|Default|GetMaxFailPercentage))
      (Variables|Default|SetisPouringFailed true))))

(event OnComponentBeginOverlap(SLContactMonitorBox)
  (params (OverlappedComponent :type Primitive%20Component%20Object%20Reference) (OtherActor :type Actor%20Object%20Reference) (OtherComp :type Primitive%20Component%20Object%20Reference) (OtherBodyIndex :type Integer) (bFromSweep :type Boolean) (SweepResult :type Hit%20Result%20Structure%20%28by%20ref%29)))

(event OnComponentEndOverlap(SLContactMonitorBox)
  (params (OverlappedComponent :type Primitive%20Component%20Object%20Reference) (OtherActor :type Actor%20Object%20Reference) (OtherComp :type Primitive%20Component%20Object%20Reference) (OtherBodyIndex :type Integer))
  (bind _dataarray (Variables|Default|GetDataArray))
  (bind _sm_blue_cup (Variables|Default|GetSM_Blue_Cup))
  (bind _sm_bigbowl (Variables|Default|GetSM_BigBowl))
  (bind _returnvalue (Transformation|GetWorldLocation _sm_blue_cup))
  (bind _returnvalue_2 (Transformation|GetWorldLocation _sm_bigbowl))
  (Utilities|Array|AppendArray _dataarray (Utilities|Array|MakeArray (Utilities|String|Append (Utilities|GetObjectName _sm_blue_cup) "," (Utilities|GetObjectName _sm_bigbowl) "," (Utilities|String|ToString(Float) (Utilities|Time|GetTimeSeconds)) "," (Utilities|String|ToString(Float) (Variables|Default|GetRotationSpeed)) "," (Utilities|String|ToString(Float) (Variables|Default|GetMaxPouringAngle)) "," (Utilities|String|ToString(Float) (.x _returnvalue)) "," (Utilities|String|ToString(Float) (.y _returnvalue)) "," (Utilities|String|ToString(Float) (.z _returnvalue)) "," (Utilities|String|ToString(Float) (.x _returnvalue_2)) "," (Utilities|String|ToString(Float) (.y _returnvalue_2)) "," (Utilities|String|ToString(Float) (.z _returnvalue_2)) "," (Utilities|String|ToString(Integer) (Variables|Default|GetNumberOfParticles)))))
  (Variables|Default|SetDataRaws _dataarray))

(event OnComponentBeginOverlap(SLContactMonitorBox1)
  (params (OverlappedComponent :type Primitive%20Component%20Object%20Reference) (OtherActor :type Actor%20Object%20Reference) (OtherComp :type Primitive%20Component%20Object%20Reference) (OtherBodyIndex :type Integer) (bFromSweep :type Boolean) (SweepResult :type Hit%20Result%20Structure%20%28by%20ref%29))
  (bind _particleshittable (Variables|Default|GetParticlesHitTable))
  (if (not (Utilities|Array|ContainsItem _particleshittable OtherComp))
    (Utilities|Array|Add _particleshittable OtherComp)
    (if (>= (/ (Math|Conversions|ToFloat(Integer) (Utilities|Array|Length (Variables|Default|GetParticlesHitTable))) (Math|Conversions|ToFloat(Integer) (Variables|Default|GetNumberOfParticles))) (Variables|Default|GetMaxFailPercentage))
      (Variables|Default|SetisPouringFailed true))))

(event OnComponentBeginOverlap(SLContactMonitorBox2)
  (params (OverlappedComponent :type Primitive%20Component%20Object%20Reference) (OtherActor :type Actor%20Object%20Reference) (OtherComp :type Primitive%20Component%20Object%20Reference) (OtherBodyIndex :type Integer) (bFromSweep :type Boolean) (SweepResult :type Hit%20Result%20Structure%20%28by%20ref%29))
  (bind _particleshittable (Variables|Default|GetParticlesHitTable))
  (if (not (Utilities|Array|ContainsItem _particleshittable OtherComp))
    (Utilities|Array|Add _particleshittable OtherComp)
    (if (>= (/ (Math|Conversions|ToFloat(Integer) (Utilities|Array|Length (Variables|Default|GetParticlesHitTable))) (Math|Conversions|ToFloat(Integer) (Variables|Default|GetNumberOfParticles))) (Variables|Default|GetMaxFailPercentage))
      (Variables|Default|SetisPouringFailed true))))

(event OnComponentBeginOverlap(SLContactMonitorBox3)
  (params (OverlappedComponent :type Primitive%20Component%20Object%20Reference) (OtherActor :type Actor%20Object%20Reference) (OtherComp :type Primitive%20Component%20Object%20Reference) (OtherBodyIndex :type Integer) (bFromSweep :type Boolean) (SweepResult :type Hit%20Result%20Structure%20%28by%20ref%29))
  (bind _particleshittable (Variables|Default|GetParticlesHitTable))
  (if (not (Utilities|Array|ContainsItem _particleshittable OtherComp))
    (Utilities|Array|Add _particleshittable OtherComp)
    (if (>= (/ (Math|Conversions|ToFloat(Integer) (Utilities|Array|Length (Variables|Default|GetParticlesHitTable))) (Math|Conversions|ToFloat(Integer) (Variables|Default|GetNumberOfParticles))) (Variables|Default|GetMaxFailPercentage))
      (Variables|Default|SetisPouringFailed true))))

(event EventBeginPlay
  (bind _savegamename (Variables|Default|GetSaveGameName))
  (Variables|Default|SetLastTimeStamp (Utilities|Time|GetTimeSeconds))
  (Utilities|Array|Clear (Variables|Default|GetParticlesHitTable))
  (Variables|Default|SetisEndTimeSet false)
  (Variables|Default|SetisStartTimeSet false)
  (if (Variables|Default|GetLoadCSV)
    (bind _returnvalue (SaveGame|DoesSaveGameExist (Variables|Default|GetSaveGameName)))
    (if _returnvalue
      (bind _returnvalue_2 (SaveGame|LoadGamefromSlot (Variables|Default|GetSaveGameName)))
      (bind _asmy_save_game (Utilities|Casting|CastToMySaveGame _returnvalue_2))
      (Variables|Default|SetSaveGame _asmy_save_game)
      (else
        (bind _returnvalue_3 (SaveGame|CreateSaveGameObject "/Game/Maps/Simulation/MySaveGame.MySaveGame_C"))
        (bind _output_get (Variables|Default|SetSaveGame _returnvalue_3))
        (Variables|/Game/Maps/Simulation/MySaveGame.MySaveGame_C|SetLine _output_get 0)
        (Variables|/Game/Maps/Simulation/MySaveGame.MySaveGame_C|SetCurrentTrial _output_get 0)))
    (bind _outfilecontents (Class|CSVtoStruct|LoadCSV (Variables|Default|GetCSVFilePath) :!label _label))
    (if (< (Variables|/Game/Maps/Simulation/MySaveGame.MySaveGame_C|GetLine (Variables|Default|GetSaveGame)) (Utilities|Array|Length _outfilecontents))
      (Variables|Default|SetMaxPouringAngle (Math|Conversions|ToFloat(Integer) (Utilities|Array|Get(acopy) (Utilities|String|ParseIntoArray (Utilities|Array|Get(acopy) _outfilecontents (Variables|/Game/Maps/Simulation/MySaveGame.MySaveGame_C|GetLine (Variables|Default|GetSaveGame))) ","))))
      (Variables|Default|SetRotationSpeed (Math|Conversions|ToFloat(Integer) (Utilities|Array|Get(acopy) (Utilities|String|ParseIntoArray (Utilities|Array|Get(acopy) _outfilecontents (Variables|/Game/Maps/Simulation/MySaveGame.MySaveGame_C|GetLine (Variables|Default|GetSaveGame))) ",") 1)))
      (Variables|Default|SetMaxIterations (Math|Conversions|ToInteger(Byte) (Utilities|Array|Get(acopy) (Utilities|String|ParseIntoArray (Utilities|Array|Get(acopy) _outfilecontents (Variables|/Game/Maps/Simulation/MySaveGame.MySaveGame_C|GetLine (Variables|Default|GetSaveGame))) ",") 2)))
      (bind _result (Math|Integer|IncrementInt (Variables|/Game/Maps/Simulation/MySaveGame.MySaveGame_C|GetCurrentTrial (Variables|Default|GetSaveGame)))
        (:%20%20
          (if (> _result (Variables|Default|GetMaxIterations))
            (Math|Integer|IncrementInt (Variables|/Game/Maps/Simulation/MySaveGame.MySaveGame_C|GetLine (Variables|Default|GetSaveGame))
              (:%20%20
                (Variables|/Game/Maps/Simulation/MySaveGame.MySaveGame_C|SetCurrentTrial (Variables|Default|GetSaveGame) 0)
                (goto _label)))
            (else
              (SaveGame|SaveGametoSlot (Variables|Default|GetSaveGame) (Variables|Default|GetSaveGameName))))))
      (else
        (SaveGame|DeleteGameinSlot (Variables|Default|GetSaveGameName))
        (Game|QuitGame 0 "Quit" false)))
    (elif (Variables|Default|GetUseSaveGameScript)
      (bind _returnvalue_4 (SaveGame|DoesSaveGameExist _savegamename))
      (if _returnvalue_4
        (bind _returnvalue_5 (SaveGame|LoadGamefromSlot (Variables|Default|GetSaveGameName)))
        (bind _asmy_save_game_2 (Utilities|Casting|CastToMySaveGame _returnvalue_5))
        (bind _output_get_2 (Variables|Default|SetSaveGame _asmy_save_game_2))
        (Math|Integer|IncrementInt (Variables|/Game/Maps/Simulation/MySaveGame.MySaveGame_C|GetCurrentTrial _output_get_2)
          (:%20%20
            (Variables|Default|SetRotationSpeed (Variables|/Game/Maps/Simulation/MySaveGame.MySaveGame_C|GetRotationSpeed _output_get_2))
            (bind _output_get_3 (Variables|Default|SetMaxPouringAngle (Variables|/Game/Maps/Simulation/MySaveGame.MySaveGame_C|GetCurrentPouringAngle _output_get_2)))
            (if (>= (Variables|/Game/Maps/Simulation/MySaveGame.MySaveGame_C|GetCurrentTrial (Variables|Default|GetSaveGame)) (Variables|Default|GetMaxIterations))
              (Variables|/Game/Maps/Simulation/MySaveGame.MySaveGame_C|SetCurrentTrial (Variables|Default|GetSaveGame) 0)
              (bind _output_get_4 (Variables|Default|SetMaxPouringAngle (+ (Variables|Default|GetIncreasePouringAngleBy) _output_get_3)))
              (if (> _output_get_4 (Variables|Default|GetEndMaxPouringAngle))
                (Variables|Default|SetMaxPouringAngle (Variables|/Game/Maps/Simulation/MySaveGame.MySaveGame_C|GetStartPouringAngle (Variables|Default|GetSaveGame)))
                (Variables|/Game/Maps/Simulation/MySaveGame.MySaveGame_C|SetCurrentPouringAngle (Variables|Default|GetSaveGame) (Variables|/Game/Maps/Simulation/MySaveGame.MySaveGame_C|GetStartPouringAngle (Variables|Default|GetSaveGame)))
                (bind _output_get_5 (Variables|Default|SetRotationSpeed (+ (Variables|Default|GetRotationSpeed) (Variables|Default|GetIncreaseRotationSpeedBy))))
                (bind _output_get_6 (Variables|/Game/Maps/Simulation/MySaveGame.MySaveGame_C|SetRotationSpeed (Variables|Default|GetSaveGame) _output_get_5))
                (if (> _output_get_6 (Variables|Default|GetMaxRotationSpeed))
                  (SaveGame|DeleteGameinSlot (Variables|Default|GetSaveGameName))
                  (Game|QuitGame 0 "Quit" false)
                  (else
                    (SaveGame|SaveGametoSlot (Variables|Default|GetSaveGame) (Variables|Default|GetSaveGameName) :!label _label_2)))
                (else
                  (Variables|/Game/Maps/Simulation/MySaveGame.MySaveGame_C|SetCurrentPouringAngle (Variables|Default|GetSaveGame) _output_get_4)
                  (goto _label_2)))
              (else
                (goto _label_2)))))
        (else
          (bind _returnvalue_6 (SaveGame|CreateSaveGameObject "/Game/Maps/Simulation/MySaveGame.MySaveGame_C"))
          (bind _output_get_7 (Variables|Default|SetSaveGame _returnvalue_6))
          (Variables|/Game/Maps/Simulation/MySaveGame.MySaveGame_C|SetCurrentTrial _output_get_7 0)
          (Variables|/Game/Maps/Simulation/MySaveGame.MySaveGame_C|SetCurrentPouringAngle _output_get_7 (Variables|Default|GetMaxPouringAngle))
          (Variables|/Game/Maps/Simulation/MySaveGame.MySaveGame_C|SetStartPouringAngle _output_get_7 (Variables|Default|GetMaxPouringAngle))
          (Variables|/Game/Maps/Simulation/MySaveGame.MySaveGame_C|SetRotationSpeed _output_get_7 (Variables|Default|GetRotationSpeed))
          (SaveGame|SaveGametoSlot (Variables|Default|GetSaveGame) (Variables|Default|GetSaveGameName))))
      (else
        (SaveGame|DeleteGameinSlot _savegamename)))))

(event Collision|EventActorBeginOverlap
  (params (OtherActor :type Actor%20Object%20Reference)))

(event EventTick
  (params (DeltaSeconds :type Float%20%28single-precision%29))
  (bind _sm_blue_cup (Variables|Default|GetSM_Blue_Cup))
  (if (Variables|Default|GetParticlesFilled)
    (if (> (- (Utilities|Time|GetTimeSeconds) (Variables|Default|GetTestTime)) 0.0)
      (Variables|Default|SetfailedParticleAmount (Utilities|Array|Length (Variables|Default|GetParticlesHitTable)))
      (bind _output_get (Variables|Default|SetcurrentRotationAngle (.roll (Variables|/Script/Engine.SceneComponent|GetRelativeRotation _sm_blue_cup))))
      (if (Math|Float|InRange(Float) _output_get 0.0 (Variables|Default|GetMaxPouringAngle))
        (if (Variables|Default|GetisStartTimeSet)
          (CallFunction|CheckRotationTime)
          (else
            (bind _output_get_2 (Variables|Default|SetStartTime (Utilities|Time|GetTimeSeconds)))
            (Variables|Default|SetisStartTimeSet true)
            (if (Variables|Default|GetisFillingBlueprint)
              (Variables|Default|SetstartTimeStamp _output_get_2))))
        (Transformation|AddRelativeRotation _sm_blue_cup (Math|Rotator|MakeRotator (* (Utilities|Time|GetWorldDeltaSeconds) (Variables|Default|GetRotationSpeed)) 0.0 0.0) false false)
        (else
          (Utilities|FlowControl|Delay 2.0)
          (Development|ExecuteConsoleCommand "RestartLevel" 0))))
    (else
      (CallFunction|DropParticle)
      (Variables|Default|SetTestTime (Utilities|Time|GetTimeSeconds)))))

(fn ConstructionScript
  (LocalVariables|SetCountParticles 0)
  (for _array_element (Components|GetChildrenComponents (Variables|Default|GetDefaultSceneRoot) true)
    (if (Utilities|String|StartsWith (Utilities|GetObjectName _array_element) "particle")
      (Math|Integer|IncrementInt (LocalVariables|GetCountParticles))))
  (Variables|Default|SetNumberOfParticles (LocalVariables|GetCountParticles)))

(fn CheckRotationTime
  (if (not (Math|Float|InRange(Float) (Variables|Default|GetcurrentRotationAngle) 0.0 45.0))
    (if (not (Variables|Default|GetisEndTimeSet))
      (Variables|Default|SetisEndTimeSet true)
      (Variables|Default|SettimeElapsed (- (Utilities|Time|GetTimeSeconds) (Variables|Default|GetStartTime)))
      (Variables|Default|SetturnedDegrees 45.0))))

(fn DropParticle
  (bind _spawningbox (Variables|Default|GetSpawningBox))
  (Variables|Default|SetisFillingBlueprint true)
  (if (>= (- (Utilities|Time|GetTimeSeconds) (Variables|Default|GetLastTimeStamp)) 0.1)
    (Variables|Default|SetLastTimeStamp (Utilities|Time|GetTimeSeconds))
    (bind _returnvalue (AddComponent|AddStaticMeshComponent false (Math|Transform|MakeTransform (Math|Random|RandomPointinBoundingBox (Variables|/Script/Engine.SceneComponent|GetRelativeLocation _spawningbox) (Variables|/Script/Engine.BoxComponent|GetBoxExtent _spawningbox)))))
    (Physics|SetSimulatePhysics _returnvalue true)
    (Components|StaticMesh|SetStaticMesh _returnvalue "/Game/Models/Misc/PouringParticle/SM_PouringParticle.SM_PouringParticle")
    (Class|PrimitiveComponent|SetLinearDamping _returnvalue 1.0)
    (Class|PrimitiveComponent|SetAngularDamping _returnvalue 1.0)
    (Collision|SetCollisionProfileName _returnvalue "BlockAll" true :!class /Script/Engine.PrimitiveComponent)
    (Class|PrimitiveComponent|SetPhysMaterialOverride _returnvalue "/Engine/EngineMaterials/PhysMat_Carboard.PhysMat_Carboard")
    (Math|Integer|IncrementInt (Variables|Default|GetAddedParticles)
      (:%20%20
        (if (>= (Variables|Default|GetAddedParticles) (Variables|Default|GetParticles))
          (Variables|Default|SetParticlesFilled true))))))

(fn DeleteSavegame
  (SaveGame|DeleteGameinSlot (Variables|Default|GetSaveGameName)))