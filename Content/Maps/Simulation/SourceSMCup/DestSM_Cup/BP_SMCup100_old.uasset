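; Pouring-simulation actor that tilts a source cup and records data about particles poured toward a destination cup.
; Tick rolls SMCup while its angle is within MaxPouringAngle; each end-overlap on the main contact box appends a CSV row of time, rotation and both cup positions.
; Four other contact boxes share a table of unique hits, flagging failure once it reaches MaxFailPercentage of the particle components counted by name at construction.
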(event OnComponentBeginOverlap(SLContactMonitorBox4)
  (params (OverlappedComponent :type Primitive%20Component%20Object%20Reference) (OtherActor :type Actor%20Object%20Reference) (OtherComp :type Primitive%20Component%20Object%20Reference) (OtherBodyIndex :type Integer) (bFromSweep :type Boolean) (SweepResult :type Hit%20Result%20Structure%20%28by%20ref%29))
  (bind _particleshittable (Variables|Default|GetParticlesHitTable))
  (if (not (Utilities|Array|ContainsItem _particleshittable OtherComp))
    (Utilities|Array|Add _particleshittable 0)
    (if (>= (/ (Math|Conversions|ToFloat(Integer) (Utilities|Array|Length (Variables|Default|GetParticlesHitTable))) (Math|Conversions|ToFloat(Integer) (Variables|Default|GetNumberOfParticles))) (Variables|Default|GetMaxFailPercentage))
      (Variables|Default|SetisPouringFailed true))))

(event OnComponentBeginOverlap(SLContactMonitorBox)
  (params (OverlappedComponent :type Primitive%20Component%20Object%20Reference) (OtherActor :type Actor%20Object%20Reference) (OtherComp :type Primitive%20Component%20Object%20Reference) (OtherBodyIndex :type Integer) (bFromSweep :type Boolean) (SweepResult :type Hit%20Result%20Structure%20%28by%20ref%29)))

(event OnComponentEndOverlap(SLContactMonitorBox)
  (params (OverlappedComponent :type Primitive%20Component%20Object%20Reference) (OtherActor :type Actor%20Object%20Reference) (OtherComp :type Primitive%20Component%20Object%20Reference) (OtherBodyIndex :type Integer))
  (bind _dataarray (Variables|Default|GetDataArray))
  (bind _sm_cup (Variables|Default|GetSM_Cup))
  (bind _sm_cup_dest (Variables|Default|GetSM_Cup_Dest))
  (bind _returnvalue (Transformation|GetWorldLocation _sm_cup))
  (bind _returnvalue_2 (Transformation|GetWorldLocation _sm_cup_dest))
  (Utilities|Array|AppendArray _dataarray (Utilities|Array|MakeArray (Utilities|String|Append (Utilities|GetObjectName _sm_cup) "," (Utilities|GetObjectName (Variables|Default|GetSM_Cup_Dest)) "," (Utilities|String|ToString(Float) (Utilities|Time|GetTimeSeconds)) "," (Utilities|String|ToString(Float) (Variables|Default|GetRotationSpeed)) "," (Utilities|String|ToString(Float) (.roll (Variables|/Script/Engine.SceneComponent|GetRelativeRotation _sm_cup))) "," (Utilities|String|ToString(Float) (.x _returnvalue)) "," (Utilities|String|ToString(Float) (.y _returnvalue)) "," (Utilities|String|ToString(Float) (.z _returnvalue)) "," (Utilities|String|ToString(Float) (.x _returnvalue_2)) "," (Utilities|String|ToString(Float) (.y _returnvalue_2)) "," (Utilities|String|ToString(Float) (.z _returnvalue_2)) "," "132")))
  (Variables|Default|SetDataRaws _dataarray))

(event OnComponentBeginOverlap(SLContactMonitorBox1)
  (params (OverlappedComponent :type Primitive%20Component%20Object%20Reference) (OtherActor :type Actor%20Object%20Reference) (OtherComp :type Primitive%20Component%20Object%20Reference) (OtherBodyIndex :type Integer) (bFromSweep :type Boolean) (SweepResult :type Hit%20Result%20Structure%20%28by%20ref%29))
  (bind _particleshittable (Variables|Default|GetParticlesHitTable))
  (if (not (Utilities|Array|ContainsItem _particleshittable OtherComp))
    (Utilities|Array|Add _particleshittable 0)
    (if (>= (/ (Math|Conversions|ToFloat(Integer) (Utilities|Array|Length (Variables|Default|GetParticlesHitTable))) (Math|Conversions|ToFloat(Integer) (Variables|Default|GetNumberOfParticles))) (Variables|Default|GetMaxFailPercentage))
      (Variables|Default|SetisPouringFailed true))))

(event OnComponentBeginOverlap(SLContactMonitorBox2)
  (params (OverlappedComponent :type Primitive%20Component%20Object%20Reference) (OtherActor :type Actor%20Object%20Reference) (OtherComp :type Primitive%20Component%20Object%20Reference) (OtherBodyIndex :type Integer) (bFromSweep :type Boolean) (SweepResult :type Hit%20Result%20Structure%20%28by%20ref%29))
  (bind _particleshittable (Variables|Default|GetParticlesHitTable))
  (if (not (Utilities|Array|ContainsItem _particleshittable OtherComp))
    (Utilities|Array|Add _particleshittable 0)
    (if (>= (/ (Math|Conversions|ToFloat(Integer) (Utilities|Array|Length (Variables|Default|GetParticlesHitTable))) (Math|Conversions|ToFloat(Integer) (Variables|Default|GetNumberOfParticles))) (Variables|Default|GetMaxFailPercentage))
      (Variables|Default|SetisPouringFailed true))))

(event OnComponentBeginOverlap(SLContactMonitorBox3)
  (params (OverlappedComponent :type Primitive%20Component%20Object%20Reference) (OtherActor :type Actor%20Object%20Reference) (OtherComp :type Primitive%20Component%20Object%20Reference) (OtherBodyIndex :type Integer) (bFromSweep :type Boolean) (SweepResult :type Hit%20Result%20Structure%20%28by%20ref%29))
  (bind _particleshittable (Variables|Default|GetParticlesHitTable))
  (if (not (Utilities|Array|ContainsItem _particleshittable OtherComp))
    (Utilities|Array|Add _particleshittable 0)
    (if (>= (/ (Math|Conversions|ToFloat(Integer) (Utilities|Array|Length (Variables|Default|GetParticlesHitTable))) (Math|Conversions|ToFloat(Integer) (Variables|Default|GetNumberOfParticles))) (Variables|Default|GetMaxFailPercentage))
      (Variables|Default|SetisPouringFailed true))))

(event EventBeginPlay
  (Utilities|Array|Clear (Variables|Default|GetParticlesHitTable)))

(event Collision|EventActorBeginOverlap
  (params (OtherActor :type Actor%20Object%20Reference)))

(event EventTick
  (params (DeltaSeconds :type Float%20%28single-precision%29))
  (if (Math|Float|InRange(Float) (.roll (Variables|/Script/Engine.SceneComponent|GetRelativeRotation (Variables|Default|GetSM_Cup))) 0.0 (Variables|Default|GetMaxPouringAngle))
    (Transformation|AddRelativeRotation (Variables|Default|GetSM_Cup) (Math|Rotator|MakeRotator (Variables|Default|GetRotationSpeed) 0.0 0.0) false false)))

(fn ConstructionScript
  (Variables|Default|SetNumberOfParticles 0)
  (for _array_element (Components|GetChildrenComponents (Variables|Default|GetDefaultSceneRoot) true)
    (if (Utilities|String|StartsWith (Utilities|GetObjectName _array_element) "particle")
      (Math|Integer|IncrementInt (Variables|Default|GetNumberOfParticles)))))